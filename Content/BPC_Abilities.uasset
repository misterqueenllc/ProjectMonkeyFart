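; BPC_Abilities is an early-stage component that handles attack and ability selection for a CH_PerformerBase character.
; On BeginPlay it casts its owner to CH_PerformerBase and caches it as Parent.
; BasicAttack sets the parent's Attacks enum when the UpDown axis is at least 0.2; checks for the other three directions are unconnected.
; SwitchAbility switches on the parent's AbilityType but has no case logic yet.
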(event Custom|SwitchAbility
  (switch Utilities|FlowControl|Switch|SwitchonE_AbilityTypes (Variables|/Game/Blueprints/Player/Performers/CH_PerformerBase.CH_PerformerBase_C|GetAbilityType (Variables|Default|GetParent))))

(event Custom|Basic%20Attack
  (if (>= (Variables|/Game/Blueprints/Player/Performers/CH_PerformerBase.CH_PerformerBase_C|GetUpDown (Variables|Default|GetParent)) 0.2)
    (Variables|/Game/Blueprints/Player/Performers/CH_PerformerBase.CH_PerformerBase_C|SetAttacks (Variables|Default|GetParent) "NewEnumerator0")))

(event EventBeginPlay
  ;[1 1 0] GetOwner
  (bind _asch_performer_base (Utilities|Casting|CastToCH_PerformerBase (Components|GetOwner)))
  (Variables|Default|SetParent _asch_performer_base))