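; Base projectile for fighters that flies along Y, drops by Gravity and hits other performers.
; Tick teleports the mesh by fixed per-frame steps without delta time or sweep (ZSpeed is unused), and calls EndLifeTime after a LifeTime delay.
; Sphere overlap with a non-owner performer's capsule applies the DTAttack row for AttackName, always passing Left as hit direction.
; Hit, expiry, ground, wall and absorb events are empty hooks; reflection negates both speeds.
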(event OnComponentBeginOverlap(Sphere)
  (params (OverlappedComponent :type Primitive%20Component%20Object%20Reference) (OtherActor :type Actor%20Object%20Reference) (OtherComp :type Primitive%20Component%20Object%20Reference) (OtherBodyIndex :type Integer) (bFromSweep :type Boolean) (SweepResult :type Hit%20Result%20Structure%20%28by%20ref%29))
  ;[1 1 0 1 30] Overlap fighters
  (bind _asbp_performer_base (Utilities|Casting|CastToBP_PerformerBase OtherActor))
  (if (and (== (Variables|/Script/Engine.Character|GetCapsuleComponent _asbp_performer_base) OtherComp) (!= _asbp_performer_base (Components|GetOwner)))
    (bind _returnvalue (Utilities|GetDataTableRow (Variables|/Game/Blueprints/Player/BP_PerformerBase.BP_PerformerBase_C|GetDT_Attack (Variables|Default|GetParent)) (Variables|Default|GetAttackName))
      (:then
        (Default|Hit _asbp_performer_base "NewEnumerator0" (.Damage (Utilities|Struct|BreakF_Attacks _returnvalue)) 0 (Math|Float|Truncate (.BaseKnock (Utilities|Struct|BreakF_Attacks _returnvalue))) (.Scale (Utilities|Struct|BreakF_Attacks _returnvalue)) (.Angle (Utilities|Struct|BreakF_Attacks _returnvalue)) (.HitStop (Utilities|Struct|BreakF_Attacks _returnvalue)) (.HitStun (Utilities|Struct|BreakF_Attacks _returnvalue)) (Variables|Default|GetParent))
        (CallFunction|HitEvent))
      (:RowNotFound
        (Development|PrintString "NoAttackFound" true true "(R=1.000000,G=0.000000,B=0.000000,A=1.000000)" 1e+01)))))

(event Custom|EndLifeTime
  ;[1 1 0 1 30] Even Calls
)

(event Custom|SetSpeed
  (params (YSpeed :type Float%20%28single-precision%29) (XSpeed :type Float%20%28single-precision%29))
  ;[1 1 0 1 30] Even Calls
  (Variables|Default|SetYSpeed YSpeed)
  (Variables|Default|SetZSpeed XSpeed))

(event Custom|AbsorbedEvent
  ;[1 1 0 1 30] Even Calls
)

(event Custom|HitEvent
  ;[1 1 0 1 30] Even Calls
)

(event Custom|HitGroundEvent
  ;[1 1 0 1 30] Even Calls
)

(event Custom|HitWallEvent
  ;[1 1 0 1 30] Even Calls
)

(event Custom|ReflectedEvent
  ;[1 1 0 1 30] Even Calls
  (Variables|Default|SetYSpeed (* (Variables|Default|GetYSpeed) -1.0))
  (Variables|Default|SetZSpeed (* (Variables|Default|GetZSpeed) -1.0)))

(event EventTick
  (params (DeltaSeconds :type Float%20%28single-precision%29))
  ;[1 1 0 1 30] Tick
  (Utilities|FlowControl|Sequence
    (:then_0
      (Utilities|FlowControl|Delay (Variables|Default|GetLifeTime))
      (CallFunction|EndLifeTime))
    (:then_1
      (CallFunction|FGravity)
      (CallFunction|FMoveinDirection))))

(fn ConstructionScript)

(fn FGravity
  (bind _mesh (Variables|Default|GetMesh))
  (bind _returnvalue (Transformation|GetWorldLocation _mesh))
  (bind (_x _y _z) (Math|Vector|BreakVector _returnvalue))
  (Transformation|SetWorldLocation _mesh (Math|Vector|MakeVector _x _y (- _z (Variables|Default|GetGravity))) false false))

(fn FMoveinDirection
  (bind _mesh (Variables|Default|GetMesh))
  (bind _returnvalue (Transformation|GetWorldLocation _mesh))
  (bind _returnvalue_2 (Transformation|GetWorldLocation _mesh))
  (bind (_x _y _z) (Math|Vector|BreakVector _returnvalue))
  (bind (_x_2 _y_2 _z_2) (Math|Vector|BreakVector _returnvalue_2))
  (switch Utilities|FlowControl|Switch|SwitchonE_Facing (Variables|Default|GetDirection)
    (:NewEnumerator0
      (Transformation|SetWorldLocation _mesh (Math|Vector|MakeVector _x_2 (+ _y_2 (Variables|Default|GetYSpeed)) _z_2) false false))
    (:NewEnumerator1
      (Transformation|SetWorldLocation _mesh (Math|Vector|MakeVector _x (- _y (Variables|Default|GetYSpeed)) _z) false false))))