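; BP_CameraVolume is a level object that defines a rectangular camera region in the Y-Z plane from a Box component.
; On BeginPlay it derives and stores the box's top, bottom, left and right bounds from its world location and extent, ignoring rotation.
; It then moves the T, B, L and R components to those edge midpoints at the box's X position.
; The construction script is empty.
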(event EventBeginPlay
  (bind _box (Variables|Default|GetBox))
  (bind _returnvalue (Transformation|GetWorldLocation _box))
  (bind _boxextent (Variables|/Script/Engine.BoxComponent|GetBoxExtent _box))
  (bind (_x _y _z) (Math|Vector|BreakVector _boxextent))
  (bind (_x_2 _y_2 _z_2) (Math|Vector|BreakVector _returnvalue))
  (Variables|Default|SetXpos _x_2)
  (Variables|Default|SetTop (+ _z_2 _z))
  (Variables|Default|SetLeft (- _y_2 _y))
  (Variables|Default|SetRight (+ _y_2 _y))
  (Variables|Default|SetBottom (- _z_2 _z))
  (Transformation|SetWorldLocation (Variables|Default|GetT) (Math|Vector|MakeVector (Variables|Default|GetXpos) _y_2 (Variables|Default|GetTop)) false false)
  (Transformation|SetWorldLocation (Variables|Default|GetR) (Math|Vector|MakeVector (Variables|Default|GetXpos) (Variables|Default|GetRight) _z_2) false false)
  (Transformation|SetWorldLocation (Variables|Default|GetL) (Math|Vector|MakeVector (Variables|Default|GetXpos) (Variables|Default|GetLeft) _z_2) false false)
  (Transformation|SetWorldLocation (Variables|Default|GetB) (Math|Vector|MakeVector (Variables|Default|GetXpos) _y_2 (Variables|Default|GetBottom)) false false))

(fn ConstructionScript)