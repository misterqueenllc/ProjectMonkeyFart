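; BP_Platform is a level platform that performers stand on from above and pass through from below or while phasing.
; On BeginPlay, its Number assigns the cube one of five custom collision channels, printing warnings for invalid numbers.
; Every Tick, it loops over all BP_PerformerBase actors and sets each capsule's response to that channel: Block when FootZPosition is above the platform and PlatPhaze is off, otherwise Ignore.
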(event EventBeginPlay
  (bind _cube (Variables|Default|GetCube))
  ;[1 1 1 1 25] Set Collision Channle
  (switch int (Variables|Default|GetNumber)
    (:Default
      (Development|PrintString "SET PLATFORM NUMBER!" true true "(R=1.000000,G=0.000000,B=0.130888,A=1.000000)"))
    (:0
      (Collision|SetCollisionObjectType _cube "ECC_GameTraceChannel1")
      (Variables|Default|SetPlatform "ECC_GameTraceChannel1"))
    (:1
      (Collision|SetCollisionObjectType _cube "ECC_GameTraceChannel2")
      (Variables|Default|SetPlatform "ECC_GameTraceChannel2"))
    (:2
      (Collision|SetCollisionObjectType _cube "ECC_GameTraceChannel3")
      (Variables|Default|SetPlatform "ECC_GameTraceChannel3"))
    (:3
      (Collision|SetCollisionObjectType _cube "ECC_GameTraceChannel4")
      (Variables|Default|SetPlatform "ECC_GameTraceChannel4"))
    (:4
      (Collision|SetCollisionObjectType _cube "ECC_GameTraceChannel5")
      (Variables|Default|SetPlatform "ECC_GameTraceChannel5"))
    (:5
      (Development|PrintString "EXCEEDED VALUE RANGE FOR PLATFORMS! ADD NEW COLLISION CHANNELS " true true "(R=1.000000,G=0.000000,B=0.130888,A=1.000000)"))))

(event EventTick
  (params (DeltaSeconds :type Float%20%28single-precision%29))
  (bind _platform (Variables|Default|GetPlatform))
  ;[1 1 1 1 25] Comment
  (Variables|Default|SetZPosition (.Z (Math|Vector|BreakVector (Transformation|GetActorLocation))))
  (bind _outactors (Actor|GetAllActorsOfClass "/Game/Blueprints/Player/BP_PerformerBase.BP_PerformerBase_C"))
  (for _array_element _outactors
    (if (> (Variables|/Game/Blueprints/Player/BP_PerformerBase.BP_PerformerBase_C|GetFootZPosition _array_element) (Variables|Default|GetZPosition))
      (if (not (Variables|/Game/Blueprints/Player/BP_PerformerBase.BP_PerformerBase_C|GetPlatPhaze _array_element))
        (Collision|SetCollisionResponsetoChannel (Variables|/Script/Engine.Character|GetCapsuleComponent _array_element) _platform "ECR_Block")
        (else
          (Collision|SetCollisionResponsetoChannel (Variables|/Script/Engine.Character|GetCapsuleComponent _array_element) _platform "ECR_Ignore" :!label _label)))
      (else
        (goto _label)))))

(fn ConstructionScript)