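; BP_Respawn is a temporary respawn platform that eases down to a target height for the performer that owns it.
; It destroys itself after five seconds, or shortly after the owner gives horizontal input or enters a particular state.
; Every tick it scans all performers and sets their capsules to block the Platforms channel only when their feet are above it and they are not phasing through.
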(event Custom|Leave
  ;[1 1 1] LeavePlatform
  (bind _asbp_performer_base (Utilities|Casting|CastToBP_PerformerBase (Components|GetOwner)))
  (if (or (!= (Variables|/Game/Blueprints/Player/BP_PerformerBase.BP_PerformerBase_C|GetLeftRight _asbp_performer_base) 0.0) (Utilities|Enum|Equal(Enum) (Variables|/Game/Blueprints/Player/BP_PerformerBase.BP_PerformerBase_C|GetStates _asbp_performer_base) "NewEnumerator0"))
    (Utilities|FlowControl|Delay 0.2)
    (Actor|DestroyActor)))

(event EventTick
  (params (DeltaSeconds :type Float%20%28single-precision%29))
  (bind _returnvalue (Transformation|GetActorLocation))
  (bind (_x _y _z) (Math|Vector|BreakVector _returnvalue))
  (Utilities|FlowControl|Sequence
    (:then_0
      (CallFunction|FPhase)
      (CallFunction|Leave)
      (if (> _z (Variables|Default|GetMoveZTo))
        (Transformation|SetActorLocation (Math|Interpolation|VInterpTo _returnvalue (Math|Vector|MakeVector _x _y (Variables|Default|GetMoveZTo)) DeltaSeconds 3.0) false false)))
    (:then_1
      (Utilities|FlowControl|Delay 5.0)
      (Actor|DestroyActor))))

(fn ConstructionScript
  (Collision|SetCollisionObjectType (Variables|Default|GetCylinder) "ECC_GameTraceChannel6"))

(fn FPhase
  (bind _platforms (Variables|Default|GetPlatforms))
  (Variables|Default|SetZPos (.Z (Math|Vector|BreakVector (Transformation|GetActorLocation))))
  (bind _outactors (Actor|GetAllActorsOfClass "/Game/Blueprints/Player/BP_PerformerBase.BP_PerformerBase_C"))
  (for _array_element _outactors
    (if (> (Variables|/Game/Blueprints/Player/BP_PerformerBase.BP_PerformerBase_C|GetFootZPosition _array_element) (Variables|Default|GetZPos))
      (if (not (Variables|/Game/Blueprints/Player/BP_PerformerBase.BP_PerformerBase_C|GetPlatPhaze _array_element))
        (Collision|SetCollisionResponsetoChannel (Variables|/Script/Engine.Character|GetCapsuleComponent _array_element) _platforms "ECR_Block")
        (else
          (Collision|SetCollisionResponsetoChannel (Variables|/Script/Engine.Character|GetCapsuleComponent _array_element) _platforms "ECR_Ignore" :!label _label)))
      (else
        (goto _label)))))