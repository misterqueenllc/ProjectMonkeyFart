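; BP_DamagerInfo is a placement helper actor that records and previews a damager's location, scale, rotation and collision shape.
; Its construction script copies the transform into variables, using the root Scene's relative location, and shows that location as text.
; The CollisionShape setting toggles which of the Sphere or Box components is visible.
; At runtime it destroys itself almost immediately after BeginPlay.
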(event EventBeginPlay
  (Utilities|FlowControl|Delay 0.01)
  (Actor|DestroyActor))

(fn ConstructionScript
  (bind _scene (Variables|Default|GetScene))
  (bind _box (Variables|Default|GetBox))
  (bind _sphere (Variables|Default|GetSphere))
  (bind _relativelocation (Variables|/Script/Engine.SceneComponent|GetRelativeLocation _scene))
  (Rendering|Components|TextRender|SetText (Variables|Default|GetTextRender) (Utilities|Text|ToText(String) _relativelocation))
  (Variables|Transform|SetLocation+ _relativelocation)
  (Variables|Transform|SetScale (Transformation|GetActorScale3D))
  (Variables|Transform|SetRotation (Transformation|GetActorRotation))
  (switch Utilities|FlowControl|Switch|SwitchonE_Shapes (Variables|Default|GetCollisionShape)
    (:NewEnumerator0
      (Rendering|SetVisibility _sphere true false)
      (Rendering|SetVisibility _box false false))
    (:NewEnumerator1
      (Rendering|SetVisibility _sphere false false)
      (Rendering|SetVisibility _box true false))))