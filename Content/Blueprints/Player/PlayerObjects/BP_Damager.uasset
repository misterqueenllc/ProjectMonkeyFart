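; BP_Damager is a short-lived attack hitbox for a fighting game, with a sphere, box or capsule collision chosen at construction.
; Overlaps with valid performer collisions, filtered by ignore list, state and player number, trigger damage, knockback and hitstun from the parent's attack DataTable row, plus effects and hitstop.
; Clashing hitboxes compare Priority, destroying themselves when lower or equal.
; With a valid Parent, it destroys itself shortly after BeginPlay.
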(event OnComponentBeginOverlap(Capsule)
  (params (OverlappedComponent :type Primitive%20Component%20Object%20Reference) (OtherActor :type Actor%20Object%20Reference) (OtherComp :type Primitive%20Component%20Object%20Reference) (OtherBodyIndex :type Integer) (bFromSweep :type Boolean) (SweepResult :type Hit%20Result%20Structure%20%28by%20ref%29))
  (bind _parent (Variables|Default|GetParent))
  ;[1 1 0 1 35] Conditions
  (CallFunction|FOverlapOtherHitBox OtherActor)
  (bind _outperformer (Utilities|HitConditions OtherActor OtherComp _parent)
    (:true
      (CallFunction|OverlapServer _outperformer (Variables|Default|GetDirection) (Variables|Default|GetIgnoreList) _parent))))

(event OnComponentBeginOverlap(Box)
  (params (OverlappedComponent :type Primitive%20Component%20Object%20Reference) (OtherActor :type Actor%20Object%20Reference) (OtherComp :type Primitive%20Component%20Object%20Reference) (OtherBodyIndex :type Integer) (bFromSweep :type Boolean) (SweepResult :type Hit%20Result%20Structure%20%28by%20ref%29))
  (bind _parent (Variables|Default|GetParent))
  ;[1 1 0 1 35] Conditions
  (CallFunction|FOverlapOtherHitBox OtherActor)
  (bind _outperformer (Utilities|HitConditions OtherActor OtherComp _parent)
    (:true
      (CallFunction|OverlapServer _outperformer (Variables|Default|GetDirection) (Variables|Default|GetIgnoreList) _parent))))

(event OnComponentBeginOverlap(Sphere)
  (params (OverlappedComponent :type Primitive%20Component%20Object%20Reference) (OtherActor :type Actor%20Object%20Reference) (OtherComp :type Primitive%20Component%20Object%20Reference) (OtherBodyIndex :type Integer) (bFromSweep :type Boolean) (SweepResult :type Hit%20Result%20Structure%20%28by%20ref%29))
  (bind _parent (Variables|Default|GetParent))
  ;[1 1 0 1 35] Conditions
  (CallFunction|FOverlapOtherHitBox OtherActor)
  (bind _outperformer (Utilities|HitConditions OtherActor OtherComp _parent)
    (:true
      (CallFunction|OverlapServer _outperformer (Variables|Default|GetDirection) (Variables|Default|GetIgnoreList) _parent))))

(event Custom|IgnoreListServer
  (params (Index :type Integer) (Item :type BP%20Performer%20Base%20Object%20Reference%20%28by%20ref%29) (TargetArray :type Array%20of%20BP%20Performer%20Base%20Object%20References))
  ;[1 1 0 1 30] Ignore List
  (Utilities|Array|SetArrayElem TargetArray Index Item true))

(event Custom|OverlapServer
  (params (Target :type BP%20Performer%20Base%20Object%20Reference) (Direction :type E_Facing%20Enum :default "NewEnumerator0") (IgnoreList :type Array%20of%20BP%20Performer%20Base%20Object%20References) (Parent :type BP%20Performer%20Base%20Object%20Reference))
  ;[1 1 0 1 30] MainFuction
  (Utilities|FlowControl|DoOnce false :!label _label
    (:Completed
      (CallFunction|FOverlapPerformer Target Direction IgnoreList Parent)
      (Utilities|FlowControl|Delay 0.01)
      (goto _label Reset))))

(event Custom|OverlapClients
  (params (Target :type BP%20Performer%20Base%20Object%20Reference) (Direction :type E_Facing%20Enum :default "NewEnumerator0") (IgnoreList :type Array%20of%20BP%20Performer%20Base%20Object%20References) (Parent :type BP%20Performer%20Base%20Object%20Reference))
  ;[1 1 0 1 30] MainFuction
  (Utilities|FlowControl|DoOnce false :!label _label
    (:Completed
      (CallFunction|FOverlapPerformer Target Direction IgnoreList Parent)
      (Utilities|FlowControl|Delay 0.01)
      (goto _label Reset))))

(event Custom|IgnoreListClients
  (params (Index :type Integer) (Item :type BP%20Performer%20Base%20Object%20Reference%20%28by%20ref%29) (TargetArray :type Array%20of%20BP%20Performer%20Base%20Object%20References))
  ;[1 1 0 1 30] Ignore List
  (Utilities|Array|SetArrayElem TargetArray Index Item true))

(event Custom|DeactivateEvent
  ;[1 1 0 1 30] Events
  (Actor|DestroyActor))

(event Custom|Flinch
  ;[1 1 0 1 30] Events
  (Actor|DestroyActor))

(event EventBeginPlay
  (bind _ignorelist (Variables|Default|GetIgnoreList))
  (bind _parent (Variables|Default|GetParent))
  (bind _playernumber (Variables|/Game/Blueprints/Player/BP_PerformerBase.BP_PerformerBase_C|GetPlayerNumber _parent))
  ;[1 1 0 1 30] Events
  (Utilities|IsValid _parent
    (:Is%20Valid
      (Utilities|FlowControl|Delay 0.2)
      (Actor|DestroyActor)
      (CallFunction|IgnoreListClients _playernumber _parent _ignorelist)
      (CallFunction|IgnoreListServer _playernumber _parent _ignorelist))))

(fn ConstructionScript
  (bind _capsule (Variables|Default|GetCapsule))
  (bind _sphere (Variables|Default|GetSphere))
  (bind _box (Variables|Default|GetBox))
  (switch Utilities|FlowControl|Switch|SwitchonE_Shapes (Variables|Default|GetCollisionShape)
    (:NewEnumerator0
      (Components|DestroyComponent _box)
      (Components|DestroyComponent _capsule))
    (:NewEnumerator1
      (Components|DestroyComponent _sphere)
      (Components|DestroyComponent _capsule))
    (:NewEnumerator2
      (Components|DestroyComponent _sphere)
      (Components|DestroyComponent _box))))

(fn FOverlapOtherHitBox
  (params (Object :type Object%20Object%20Reference))
  (bind _priority (Variables|Default|GetPriority))
  (bind _asbp_damager (Utilities|Casting|CastToBP_Damager Object))
  (if (!= _asbp_damager (Components|GetOwner))
    (Utilities|IsValid _asbp_damager
      (:Is%20Valid
        (if (< _priority (Variables|BP_Damager_C|GetPriority _asbp_damager))
          (Actor|DestroyActor)
          (elif (== _priority (Variables|BP_Damager_C|GetPriority _asbp_damager))
            (CallFunction|Flinch)))))))

(fn FOverlapPerformer
  (params (Target :type BP%20Performer%20Base%20Object%20Reference) (Direction :type E_Facing%20Enum :default "NewEnumerator0") (IgnoreList :type Array%20of%20BP%20Performer%20Base%20Object%20References) (Parent :type BP%20Performer%20Base%20Object%20Reference))
  (bind _self self)
  (bind _scene (Variables|Default|GetScene _self))
  (bind _returnvalue (Transformation|GetWorldLocation _scene))
  (Utilities|Array|SetArrayElem IgnoreList (Variables|/Game/Blueprints/Player/BP_PerformerBase.BP_PerformerBase_C|GetPlayerNumber Target) Target)
  (Variables|Default|SetActive true)
  (Audio|PlaySoundatLocation _self (Variables|Default|GetHitSound) _returnvalue "0, 0, 0" 1.0 1.0 0.0 0 0 0)
  (Effects|SpawnEmitteratLocation _self (Variables|Default|GetHitParticle) _returnvalue)
  (bind _returnvalue_2 (Utilities|GetDataTableRow (Variables|/Game/Blueprints/Player/BP_PerformerBase.BP_PerformerBase_C|GetDT_Attack (Variables|Default|GetParent)) (Variables|Default|GetAttack))
    (:then
      (Default|Hit Target Direction (.Damage (Utilities|Struct|BreakF_Attacks _returnvalue_2)) (.ShieldDamage (Utilities|Struct|BreakF_Attacks _returnvalue_2)) (Math|Float|Truncate (.BaseKnock (Utilities|Struct|BreakF_Attacks _returnvalue_2))) (.Scale (Utilities|Struct|BreakF_Attacks _returnvalue_2)) (.Angle (Utilities|Struct|BreakF_Attacks _returnvalue_2)) (.HitStop (Utilities|Struct|BreakF_Attacks _returnvalue_2)) (.HitStun (Utilities|Struct|BreakF_Attacks _returnvalue_2)) Parent)
      (Default|HitStop Parent (.HitStop (Utilities|Struct|BreakF_Attacks _returnvalue_2))))
    (:RowNotFound
      (Development|PrintString "Error: AddCorrectName" true true "(R=0.562500,G=0.000000,B=0.016030,A=1.000000)"))))