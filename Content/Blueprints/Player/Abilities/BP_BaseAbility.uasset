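; Base actor for character abilities in a side-facing fighting game, with empty start, land, animation-end and projectile events for child abilities.
; While active, Tick fires start and landing hooks once, accumulates charge and ends the ability on certain Parent states.
; Helper events toggle the Parent's movement, jump, flip, attack, gravity and collision.
; Damage boxes spawn as attached BP_Damager actors per collision set, mirrored by facing; the grab-box spawn has no class set.
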(event Custom|SoftEnd
  ;[1 1 0 1 35] SoftEnd Active Ability
  (CallFunction|WalkOffLedge true)
  (Variables|Default|SetActive false)
  (CallFunction|SetFlip true)
  (CallFunction|SetJump true)
  (CallFunction|SetMovement true)
  (CallFunction|SetCanAttack true)
  (CallFunction|RemoveDamagers)
  (Variables|Default|SetInUse false))

(event Custom|SetMovement
  (params (CanMove :type Boolean))
  ;[1 1 0] Event Calls
  (Variables|/Game/Blueprints/Player/BP_PerformerBase.BP_PerformerBase_C|SetbCanMove (Variables|Default|GetParent) CanMove))

(event Custom|Land
  ;[1 1 0] Event Calls
)

(event Custom|SetCanAttack
  (params (CanAttack :type Boolean))
  ;[1 1 0] Event Calls
  (Variables|/Game/Blueprints/Player/BP_PerformerBase.BP_PerformerBase_C|SetbCanAttack (Variables|Default|GetParent) CanAttack))

(event Custom|StopAllMovement
  ;[1 1 0] Event Calls
  ;;[1 1 1 1 35] Stops Character Movement
  (Components|Movement|StopMovementImmediately (Pawn|GetMovementComponent (Variables|Default|GetParent))))

(event Custom|FreeFall
  ;[1 1 0] Event Calls
  (Variables|/Game/Blueprints/Player/BP_PerformerBase.BP_PerformerBase_C|SetStates (Variables|Default|GetParent) "NewEnumerator18"))

(event Custom|WalkOffLedge
  (params (CanWalkOff :type Boolean))
  ;[1 1 0] Event Calls
  (Variables|/Script/Engine.CharacterMovementComponent|SetbCanWalkOffLedges (Variables|/Script/Engine.Character|GetCharacterMovement (Variables|Default|GetParent)) CanWalkOff))

(event Custom|LandLag
  (params (LandAnimation :type Anim%20Montage%20Object%20Reference) (PlayRate :type Float%20%28single-precision%29) (StartPosition :type Float%20%28single-precision%29) (StartSection :type Name) (AnimNo :type Integer))
  ;[1 1 0 1 35] Landing Lag
  (CallFunction|SetFlip false)
  (CallFunction|SetJump false)
  (CallFunction|SetMovement false)
  (Animation|Montage|PlayMontage (Variables|/Script/Engine.Character|GetMesh (Variables|Default|GetParent)) LandAnimation PlayRate StartPosition StartSection
    (:OnBlendOut
      (CallFunction|SetFlip true)
      (CallFunction|SetJump false true)
      (CallFunction|SetMovement true)
      (CallFunction|EndAnim AnimNo)
      (Variables|Default|SetLanding false)
      (CallFunction|EndAbility))))

(event Custom|SetFlip
  (params (CanFlip :type Boolean))
  ;[1 1 0] Event Calls
  (Variables|/Game/Blueprints/Player/BP_PerformerBase.BP_PerformerBase_C|SetbCanFlip (Variables|Default|GetParent) CanFlip))

(event Custom|ActivateOverAbility
  (params (Ability :type BP%20Base%20Ability%20Object%20Reference))
  ;[1 1 0] Event Calls
  (bind _outactors (Actor|GetAllActorsOfClass "BP_BaseAbility_C"))
  (for _array_element _outactors
    (if (and (== _array_element Ability) (== _array_element (Components|GetOwner (Variables|Default|GetParent))))
      _)))

(event Custom|AddDamagersClient
  (params (Parent :type %20Object%20Reference))
  ;[1 1 0 1 35] Attach Damage boxes
  (CallFunction|FuncDamageBoxes Parent))

(event Custom|HitStates
  (params (State :type E_HitStates%20Enum :default "NewEnumerator0"))
  ;[1 1 0] Event Calls
  (Variables|/Game/Blueprints/Player/BP_PerformerBase.BP_PerformerBase_C|SetHitStates (Variables|Default|GetParent) State))

(event Custom|Add%20Damagers%20Server
  (params (Parent :type %20Object%20Reference))
  ;[1 1 0 1 35] Attach Damage boxes
  (CallFunction|FuncDamageBoxes Parent))

(event Custom|CharacterCollsion
  (params (NewType :type ECollisionEnabled%20Enum :default "NoCollision"))
  ;[1 1 0] Event Calls
  (Collision|SetCollisionEnabled (Variables|/Script/Engine.Character|GetCapsuleComponent (Variables|Default|GetParent)) NewType))

(event Custom|StartParticles
  (params (Attached? :type Boolean) (EmitterTemplate :type Particle%20System%20Object%20Reference) (AttachToComponent :type Scene%20Component%20Object%20Reference) (AttachPointName :type Name) (Location :type Vector) (Rotation :type Rotator) (Scale :type Vector) (LocationType :type EAttachLocation%20Enum :default "KeepRelativeOffset") (bAutoDestroy :type Boolean))
  ;[1 1 0] Event Calls
  (if Attached?
    (Effects|SpawnEmitterAttached EmitterTemplate AttachToComponent AttachPointName Location Rotation Scale LocationType bAutoDestroy)
    (else
      (Effects|SpawnEmitteratLocation EmitterTemplate Location Rotation Scale bAutoDestroy))))

(event Custom|ShootProjectile
  ;[1 1 0] Event Calls
)

(event Custom|Charge
  (params (Chargeing :type Boolean))
  ;[1 1 0] Event Calls
  (Variables|Charge|SetCharging Chargeing))

(event Custom|ChangeCollisionSet
  (params (CollisionSetInex :type Integer))
  ;[1 1 0] Event Calls
  (bind _output_get (Variables|Collisions|SetCollisionSetIndex (+ 1 (Variables|Collisions|GetCollisionSetIndex))))
  (Variables|Collisions|SetCollisionSet (Utilities|Array|Get(acopy) (Variables|Collisions|GetCollisionSetArray) _output_get)))

(event Custom|SetAttackStage
  (params (AttackStage :type Integer))
  ;[1 1 0] Event Calls
  (Variables|Default|SetAttackStage AttackStage))

(event Custom|FullBodyLedge
  (params (FullBodyLedgeGrab :type Boolean))
  ;[1 1 0] Event Calls
  (Variables|/Game/Blueprints/Player/BP_PerformerBase.BP_PerformerBase_C|SetbFullBodyLedgeGrab (Variables|Default|GetParent) FullBodyLedgeGrab))

(event Custom|AbilityStart
  ;[1 1 0] Event Calls
)

(event Custom|EndAnim
  (params (AnimNo :type Integer))
  ;[1 1 0] Event Calls
)

(event Custom|DodgeDelay
  ;[1 1 0] Event Calls
  (Default|DodgeDelayEvent (Variables|Default|GetParent)))

(event Custom|RemoveDamagers
  ;[1 1 0 1 35] Remove Damagers
  (bind _outactors (Actor|GetAllActorsOfClass "/Game/Blueprints/Player/PlayerObjects/BP_Damager.BP_Damager_C"))
  (for _array_element _outactors
    (if (== (Variables|/Game/Blueprints/Player/PlayerObjects/BP_Damager.BP_Damager_C|GetParent _array_element) (Variables|Default|GetParent))
      (Actor|DestroyActor _array_element))))

(event Custom|TickRep
  (bind _parent (Variables|Default|GetParent))
  (bind _states (Variables|/Game/Blueprints/Player/BP_PerformerBase.BP_PerformerBase_C|GetStates _parent))
  ;[1 1 0] Tick
  (if (Variables|Default|GetActive)
    (Utilities|FlowControl|Sequence
      (:then_0
        (if (not (Variables|Default|GetInUse))
          (CallFunction|AbilityStart)
          (Variables|Default|SetInUse true)))
      (:then_1
        (if (Variables|/Game/Blueprints/Player/BP_PerformerBase.BP_PerformerBase_C|GetbLanded _parent)
          (Utilities|FlowControl|DoOnce false :!label _label
            (:Completed
              (Variables|Default|SetLanding true)
              (CallFunction|Land)))
          (else
            (goto _label Reset))))
      (:then_2
        (CallFunction|FCharging))
      (:then_3
        (if (or (Utilities|Enum|Equal(Enum) _states "NewEnumerator9") (Utilities|Enum|Equal(Enum) _states "NewEnumerator6"))
          (CallFunction|EndAbility)))
      (:then_4
        (if (Utilities|Enum|Equal(Enum) _states "NewEnumerator8")
          _)))))

(event Custom|SetGravity
  (params (Settings :type E_EnableDisable%20Enum :default "NewEnumerator0") (CustomValue :type Float%20%28single-precision%29))
  (bind _parent (Variables|Default|GetParent))
  (bind _charactermovement (Variables|/Script/Engine.Character|GetCharacterMovement _parent))
  ;[1 1 0] Event Calls
  (switch Utilities|FlowControl|Switch|SwitchonE_EnableDisable Settings
    (:NewEnumerator0
      (Variables|/Script/Engine.CharacterMovementComponent|SetGravityScale _charactermovement (Variables|/Game/Blueprints/Player/Components/BPC_BP_CharacterStats.BPC_BP_CharacterStats_C|GetDefaultGravityScale (Variables|/Game/Blueprints/Player/BP_PerformerBase.BP_PerformerBase_C|GetCharacterStats _parent))))
    (:NewEnumerator1
      (Variables|/Script/Engine.CharacterMovementComponent|SetGravityScale _charactermovement 0.0))
    (:NewEnumerator2
      (Variables|/Script/Engine.CharacterMovementComponent|SetGravityScale _charactermovement CustomValue))))

(event Custom|Reset
  ;[1 1 0 1 35] Resets Values of ability
  (Variables|Charge|SetChargeLevel 0.0)
  (Variables|Default|SetChargeRatio 0.0)
  (Variables|Charge|SetChargeLevel 0.0)
  (Variables|Charge|SetCharging false)
  (Variables|Charge|SetCharged false)
  (Variables|Default|SetInUse false)
  (Variables|Default|SetAnimNumber 1)
  (Variables|Collisions|SetCollisionSet 1)
  (Variables|Default|SetActivateCollision true)
  (CallFunction|WalkOffLedge true)
  (Variables|Collisions|SetCollisionSetIndex 0))

(event Custom|GetCollisionInfo
  ;[1 1 0] Event Calls
)

(event Custom|SetJump
  (params (bCanJump :type Boolean))
  ;[1 1 0] Event Calls
  (Variables|/Game/Blueprints/Player/BP_PerformerBase.BP_PerformerBase_C|SetbCanJump (Variables|Default|GetParent) bCanJump))

(event Custom|EndAllNonChargedAbilities
  (params (Caller :type BP%20Base%20Ability%20Object%20Reference))
  ;[1 1 0] End NC Ability
  (bind _outactors (Actor|GetAllActorsOfClass "BP_BaseAbility_C"))
  (for _array_element _outactors
    (if (Math|Boolean|ANDBoolean (== (Variables|BP_BaseAbility_C|GetParent _array_element) (Variables|Default|GetParent)) (== (Variables|BP_BaseAbility_C|GetChargeLevel _array_element) 0.0) (!= _array_element Caller))
      _)))

(event Custom|EndAbility
  (bind _parent (Variables|Default|GetParent))
  ;[1 1 0 1 35] End Active Ability
  (CallFunction|WalkOffLedge true)
  (Variables|Default|SetActive false)
  (CallFunction|SetFlip true)
  (CallFunction|SetJump true)
  (CallFunction|SetMovement true)
  (CallFunction|CharacterCollsion "QueryAndPhysics")
  (CallFunction|FullbodyLedge false)
  (if (AI|Components|NavMovement|IsFalling (Pawn|GetMovementComponent (Variables|Default|GetParent)))
    (Variables|/Game/Blueprints/Player/BP_PerformerBase.BP_PerformerBase_C|SetStates _parent "NewEnumerator5")
    (else
      (Variables|/Game/Blueprints/Player/BP_PerformerBase.BP_PerformerBase_C|SetStates _parent "NewEnumerator0")))
  (Variables|/Game/Blueprints/Player/BP_PerformerBase.BP_PerformerBase_C|SetAbilityType _parent "NewEnumerator0")
  (Variables|/Game/Blueprints/Player/BP_PerformerBase.BP_PerformerBase_C|SetAttacks _parent "NewEnumerator30")
  (Variables|Default|SetInUse false))

(event Custom|Activate%20Damagers
  (bind _parent (Variables|Default|GetParent))
  ;[1 1 0 1 35] Attach Damage boxes
  (Networking|SwitchHasAuthority
    (:Authority
      (CallFunction|AddDamagersServer _parent))
    (:Remote
      (CallFunction|AddDamagersClient _parent))))

(event EventBeginPlay
  ;[1 1 0] Event Calls
  (Variables|Default|SetDT_Attack (Variables|/Game/Blueprints/Player/BP_PerformerBase.BP_PerformerBase_C|GetDT_Attack (Variables|Default|GetParent))))

(event EventTick
  (params (DeltaSeconds :type Float%20%28single-precision%29))
  ;[1 1 0] Tick
  (CallFunction|TickRep)
  (Utilities|DebugAbilityCall 0 false))

(fn ConstructionScript)

(fn FCharging
  (if (Variables|Charge|GetCharging)
    (Variables|Charge|SetChargeLevel (+ (Variables|Charge|GetChargeLevel) (Variables|Charge|GetChargeRate)))
    (Variables|Default|SetChargeRatio (/ (Variables|Charge|GetChargeMax) (Variables|Charge|GetChargeLevel)))
    (if (>= (Variables|Charge|GetChargeLevel) (Variables|Charge|GetChargeMax))
      (Variables|Charge|SetChargeLevel (Variables|Charge|GetChargeMax))
      (Variables|Charge|SetCharged true))))

(fn FDamageBoxes
  (params (InputPin :type BP%20Performer%20Base%20Object%20Reference))
  (for (_ _array_index) (Variables|Default|GetChildDamagers)
    (if (== (Utilities|Array|Get(acopy) (Variables|Default|GetCollisionSets) _array_index) (Variables|Collisions|GetCollisionSet))
      ;[1 1 0 1 30] HitBox
      (CallFunction|FSetBoxTransform _array_index)
      (if (not (Utilities|Array|Get(acopy) (Variables|Default|GetGrabBoxes) (.Index (Utilities|GetHitProperties _array_index))))
        (bind _returnvalue (Game|SpawnActorfromClass "/Game/Blueprints/Player/PlayerObjects/BP_Damager.BP_Damager_C" (Utilities|Array|Get(acopy) (Variables|Default|GetBoxTransforms) (.Index (Utilities|GetHitProperties _array_index))) "AlwaysSpawn" 0 InputPin (.Type (Utilities|GetHitProperties _array_index)) (.Shape (Utilities|GetHitProperties _array_index)) (.Priority (Utilities|GetHitProperties _array_index)) (.Socket (Utilities|GetHitProperties _array_index)) (.Facing (Utilities|GetHitProperties _array_index)) (.PFX (Utilities|GetHitProperties _array_index)) (.Sound (Utilities|GetHitProperties _array_index)) (.Attack (Utilities|GetHitProperties _array_index)) 0))
        (bind _output_get (Variables|Default|SetHitBox _returnvalue))
        (Utilities|IsValid _output_get
          (:Is%20Valid
            (Transformation|AttachActorToActor _returnvalue (Variables|Default|GetParent) "None" "KeepWorld" "KeepWorld" "KeepWorld" true)))
        (else
          ;[0.2562 0.541 1 0.708 30] GrabBox
          (bind _returnvalue_2 (Game|SpawnActorfromClass 0 (Utilities|Array|Get(acopy) (Variables|Default|GetBoxTransforms)) "AlwaysSpawn" 0 InputPin 0 0 0))
          (Utilities|IsValid _returnvalue_2
            (:Is%20Valid
              (Transformation|AttachActorToActor (.Parent (Variables|Default|GetParent)) "None" "KeepWorld" "KeepWorld" "KeepWorld" true))))))))

(fn FSetBoxTransform
  (params (Dimension :type Integer))
  (bind _collisionboxtransforms (Variables|Default|GetCollisionBoxTransforms))
  (bind _parent (Variables|Default|GetParent))
  (bind _returnvalue (Transformation|GetActorTransform _parent))
  (bind _output (Utilities|Array|Get(acopy) _collisionboxtransforms Dimension))
  (bind _mesh (Variables|/Script/Engine.Character|GetMesh _parent))
  (bind _scale (Math|Transform|BreakTransform _returnvalue))
  (bind _returnvalue_2 (Transformation|GetSocketLocation _mesh "roorSocket"))
  (bind (_location _rotation _scale_2) (Math|Transform|BreakTransform _output))
  (bind (_x _y _z) (Math|Vector|BreakVector _location))
  (bind _returnvalue_3 (* _scale_2 _scale))
  (switch Utilities|FlowControl|Switch|SwitchonE_Facing (Variables|/Game/Blueprints/Player/BP_PerformerBase.BP_PerformerBase_C|GetFacing (Variables|Default|GetParent))
    (:NewEnumerator0
      (Utilities|Array|SetArrayElem (Variables|Default|GetBoxTransforms) Dimension (Math|Transform|MakeTransform (+ _location _returnvalue_2) _rotation _returnvalue_3) true))
    (:NewEnumerator1
      (Utilities|Array|SetArrayElem (Variables|Default|GetBoxTransforms) Dimension (Math|Transform|MakeTransform (+ (Math|Vector|MakeVector _x (* _y -1.0) _z) _returnvalue_2) _rotation _returnvalue_3) true)))
  (return))