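; Character stats component for a performer character, tracking stock count and an accumulating damage Percent.
; On BeginPlay it copies the stock count from the performance game instance when the game subtype is Stock.
; TakeDamage adds damage to Percent only while the parent's hit state is the first enum value.
; ScreenShake plays a world camera shake at the parent's location and force feedback on that player's controller.
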(event Custom|TakeDamage
  (params (Damage :type Integer))
  ;[1 1 0] TakeDamage
  (if (Utilities|Enum|Equal(Enum) (Variables|/Game/Blueprints/Player/Performers/CH_PerformerBase.CH_PerformerBase_C|GetHitStates (Variables|Default|GetParent)) "NewEnumerator0")
    (Variables|Life|SetPercent (+ Damage (Variables|Life|GetPercent)))))

(event Custom|ScreenShake
  (bind _parent (Variables|Default|GetParent))
  ;[1 1 0] ScreenShake
  (Camera|PlayWorldCameraShake 0 (Transformation|GetActorLocation _parent) 0.0 0.0)
  (Game|Feedback|PlayDynamicForceFeedback (Game|GetPlayerController (Variables|/Game/Blueprints/Player/Performers/CH_PerformerBase.CH_PerformerBase_C|GetPlayerNum _parent)) 4.0 0.3 true true true true))

(event EventBeginPlay
  ;[1 1 0] SetStock by Instance
  (bind _asgi_performance_instance (Utilities|Casting|CastToGI_PerformanceInstance (Game|GetGameInstance)))
  (Utilities|Casting|CastToCH_PerformerBase (Components|GetOwner))
  (switch Utilities|FlowControl|Switch|SwitchonE_GameSubType (Variables|/Game/Blueprints/Core/GI_PerformanceInstance.GI_PerformanceInstance_C|GetGameSubType _asgi_performance_instance)
    (:NewEnumerator0
      (Variables|Life|SetStock (Variables|/Game/Blueprints/Core/GI_PerformanceInstance.GI_PerformanceInstance_C|GetStockCount _asgi_performance_instance)))))