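; BPC_AI is an AI component for a BP_PerformerBase owner that selects another performer as its target.
; On BeginPlay it seeds a random stream, disables the owner's attack and movement, picks a random target, and sets Active after a short wait.
; GetRandomTarget rerolls when the index matches the owner's PlayerNumber.
; ClosestTarget takes the minimum of a per-index distance array, falling back to a random pick if that yields the owner.
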(event Custom|ClosestTarget
  ;[1 1 0] GetTargets
  (bind _outactors (Actor|GetAllActorsOfClass "/Game/Blueprints/Player/BP_PerformerBase.BP_PerformerBase_C"))
  (for (_array_element _array_index) _outactors
    (if (!= _array_element (Variables|Default|GetParent))
      (Utilities|Array|SetArrayElem (Variables|Default|GetDistance) _array_index (Transformation|GetDistanceTo _array_element (Variables|Default|GetParent)) true)))
  (bind _output_get (Variables|Default|SetTarget (Utilities|Array|Get(acopy) _outactors (.IndexOfMinValue (Math|Float|MinOfFloatArray (Variables|Default|GetDistance))))))
  (if (== _output_get (Variables|Default|GetParent))
    (CallFunction|GetRandomTarget)))

(event Custom|GetRandomTarget
  (bind _random (Variables|Default|GetRandom))
  ;[1 1 0] GetTargets
  (bind _outactors (Actor|GetAllActorsOfClass "/Game/Blueprints/Player/BP_PerformerBase.BP_PerformerBase_C"))
  (CallFunction|FSetRandom (Utilities|Array|Length _outactors))
  (if (== _random (Variables|/Game/Blueprints/Player/BP_PerformerBase.BP_PerformerBase_C|GetPlayerNumber (Variables|Default|GetParent)))
    (CallFunction|GetRandomTarget)
    (else
      (Variables|Default|SetTarget (Utilities|Array|Get(acopy) _outactors _random)))))

(event EventBeginPlay
  ;[1 1 0] BeginPlay
  (Variables|Default|SetStream (Math|Random|MakeRandomStream (Math|Random|RandomInteger 1000)))
  (Utilities|FlowControl|Delay 0.02)
  (bind _asbp_performer_base (Utilities|Casting|CastToBP_PerformerBase (Components|GetOwner)))
  (bind _output_get (Variables|Default|SetParent _asbp_performer_base))
  (Variables|/Game/Blueprints/Player/BP_PerformerBase.BP_PerformerBase_C|SetCanAttack _output_get false)
  (Variables|/Game/Blueprints/Player/BP_PerformerBase.BP_PerformerBase_C|SetbCanMove _output_get false)
  (CallFunction|GetRandomTarget)
  (Utilities|FlowControl|Delay 3.0)
  (Variables|Default|SetbActive true))

(fn FSetRandom
  (params (Max :type Integer))
  (Variables|Default|SetRandom (Math|Random|RandomIntegerinRangefromStream 0 Max (Variables|Default|GetStream))))