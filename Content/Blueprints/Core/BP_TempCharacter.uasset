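; Placeholder pawn that stands in for each local player until loading completes, then swaps itself for that player's chosen character.
; On BeginPlay it derives a player index from its controller's name, flags it loaded in the game mode, and self-destructs if no character is chosen.
; Once the game state reports all loaded, it spawns and possesses the character at that index's BP_Spawn, updates the camera and destroys itself.
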(event Custom|CreateCharacter
  (bind _playernumber (Variables|Default|GetPlayerNumber))
  ;[1 1 0 1 30] Create The playable characters
  (bind _outactors (Actor|GetAllActorsOfClass "/Game/Blueprints/LevelObjects/BP_Spawn.BP_Spawn_C"))
  (if (not (Utilities|Enum|Equal(Enum) (Utilities|Array|Get(acopy) (Variables|/Game/Blueprints/Core/GI_PerformanceInstance.GI_PerformanceInstance_C|GetPlayerCharacters (Variables|Default|GetGameInstance)) _playernumber) "NewEnumerator0"))
    (CallFunction|SetCharacter (Math|Transform|MakeTransform (Transformation|GetActorLocation (Utilities|Array|Get(acopy) _outactors _playernumber))))
    (bind _outactors_2 (Actor|GetAllActorsOfClass "/Game/Blueprints/LevelObjects/BP_Camera.BP_Camera_C"))
    (Default|UpdateCamera (Utilities|Array|Get(acopy) _outactors_2))
    (Actor|DestroyActor)
    (else
      (Actor|DestroyActor))))

(event Custom|MakeHud
  (bind _returnvalue (Viewport|GetViewportSize))
  (bind _playernumber (Variables|Default|GetPlayerNumber))
  (bind (_x _y) (Math|Vector2D|BreakVector2D _returnvalue))
  ;[1 1 0 1 40] MakeHUD
  (bind _returnvalue_2 (UserInterface|CreateWidget "/Game/Blueprints/HUD/InGame/UI_CharacterInfo.UI_CharacterInfo_C" 0 _playernumber 0))
  (UserInterface|Viewport|AddtoViewport _returnvalue_2 0)
  (Class|UserWidget|SetPositioninViewport _returnvalue_2 (Math|Vector2D|MakeVector2D (+ (* _playernumber (/ _x (Math|Conversions|ToFloat(Integer) (Variables|/Game/Blueprints/Core/GI_PerformanceInstance.GI_PerformanceInstance_C|GetNumberofPlayers (Variables|Default|GetGameInstance))))) 6e+01) (- _y 2e+02)) true)
  (bind _returnvalue_3 (UserInterface|CreateWidget "/Game/Blueprints/HUD/InGame/UI_PlayerName.UI_PlayerName_C" 0 _playernumber 0))
  (UserInterface|Viewport|AddtoViewport _returnvalue_3 0)
  (Class|UserWidget|SetPositioninViewport :self _returnvalue_3))

(event EventBeginPlay
  ;[1 1 0 1 30] Get GM, GI
  (Utilities|FlowControl|Delay 0.02)
  (bind _asgm_performance_mode (Utilities|Casting|CastToGM_PerformanceMode (Game|GetGameMode))
    (:then
      (Variables|Default|SetGameMode _asgm_performance_mode))
    (:CastFailed
      _))
  (bind _asgs_performance (Utilities|Casting|CastToGS_Performance (Game|GetGameState))
    (:then
      (Variables|Default|SetGameState _asgs_performance))
    (:CastFailed
      _))
  (bind _asgi_performance_instance (Utilities|Casting|CastToGI_PerformanceInstance (Game|GetGameInstance)))
  (Variables|Default|SetGameInstance _asgi_performance_instance)
  (CallFunction|SetPlayerNumber))

(event EventTick
  (params (DeltaSeconds :type Float%20%28single-precision%29))
  (bind _gamestate (Variables|Default|GetGameState))
  ;[1 1 0 1 30] Call Create Characters when all characters have loaded
  (Utilities|IsValid _gamestate
    (:Is%20Valid
      (if (Variables|/Game/Blueprints/Core/GS_Performance.GS_Performance_C|GetAllLoaded _gamestate)
        (Utilities|FlowControl|DoOnce false
          (:Completed
            (CallFunction|CreateCharacter)))))))

(fn ConstructionScript)

(fn SetPlayerNumber
  (bind _returnvalue (Pawn|GetController))
  (bind _returnvalue_2 (Utilities|GetDisplayName _returnvalue))
  ;[1 1 0 1 40] Set The player ID no based on controller
  (Utilities|ElseBranch (or (Utilities|Enum|Equal(Enum) _returnvalue_2 "BP_PerformController") (Utilities|Enum|Equal(Enum) _returnvalue_2 "BP_PerformController_C_0")) (or (Utilities|Enum|Equal(Enum) _returnvalue_2 "BP_PerformController1") (Utilities|Enum|Equal(Enum) _returnvalue_2 "BP_PerformController_C_1")) (or (Utilities|Enum|Equal(Enum) _returnvalue_2 "BP_PerformController2") (Utilities|Enum|Equal(Enum) _returnvalue_2 "BP_PerformController_C_2"))
    (:ifCondition1
      (Variables|Default|SetPlayerNumber 0))
    (:ElseIfCondition2
      (Variables|Default|SetPlayerNumber 1))
    (:ElseIfCondition3
      (Variables|Default|SetPlayerNumber 2))
    (:ElseCondition
      (Variables|Default|SetPlayerNumber 3)))
  (Utilities|Array|SetArrayElem (Variables|/Game/Blueprints/Core/GameModes/GM_PerformanceMode.GM_PerformanceMode_C|GetPlayerLoaded (Variables|Default|GetGameMode)) (Variables|Default|GetPlayerNumber) true)
  (Rendering|Components|TextRender|SetText (Variables|Default|GetTextRender) (Utilities|Text|ToText(Integer) (Variables|Default|GetPlayerNumber)))
  (if (Utilities|Enum|Equal(Enum) (Utilities|Array|Get(acopy) (Variables|/Game/Blueprints/Core/GI_PerformanceInstance.GI_PerformanceInstance_C|GetPlayerCharacters (Variables|Default|GetGameInstance)) (Variables|Default|GetPlayerNumber)) "NewEnumerator0")
    (Actor|DestroyActor)))

(fn SetCharacter
  (params (Loc :type Transform))
  (bind _playernumber (Variables|Default|GetPlayerNumber))
  ;[1 1 0 1 40] This is where you set the characters that you play as
  (switch Utilities|FlowControl|Switch|SwitchonE_Characters (Utilities|Array|Get(acopy) (Variables|/Game/Blueprints/Core/GI_PerformanceInstance.GI_PerformanceInstance_C|GetPlayerCharacters (Variables|Default|GetGameInstance)) (Variables|Default|GetPlayerNumber))
    (:NewEnumerator0
      (bind _returnvalue (Game|SpawnActorfromClass "/Game/Blueprints/Player/BP_PerformerBase.BP_PerformerBase_C" Loc "Undefined" (Pawn|GetController) _playernumber 0))
      (Pawn|Possess (Game|GetPlayerController _playernumber) _returnvalue))
    (:NewEnumerator1
      (bind _returnvalue_2 (Game|SpawnActorfromClass "/Game/Blueprints/Player/Performers/CH_Kamiya.CH_Kamiya_C" Loc "Undefined" (Pawn|GetController) _playernumber 0))
      (Pawn|Possess (Game|GetPlayerController _playernumber) _returnvalue_2))
    (:NewEnumerator2
      (bind _returnvalue_3 (Game|SpawnActorfromClass "/Game/Blueprints/Player/Performers/CH_Maxi.CH_Maxi_C" Loc "Undefined" (Pawn|GetController) _playernumber 0))
      (Pawn|Possess (Game|GetPlayerController _playernumber) _returnvalue_3))
    (:NewEnumerator3
      (bind _returnvalue_4 (Game|SpawnActorfromClass "/Game/Blueprints/Player/Performers/CH_Rydyr.CH_Rydyr_C" Loc "Undefined" (Pawn|GetController) _playernumber 0))
      (Pawn|Possess (Game|GetPlayerController _playernumber) _returnvalue_4))
    (:NewEnumerator4
      (bind _returnvalue_5 (Game|SpawnActorfromClass "/Game/Blueprints/Player/BP_PerformerBase.BP_PerformerBase_C" Loc "Undefined" (Pawn|GetController) _playernumber 0))
      (Pawn|Possess (Game|GetPlayerController _playernumber) _returnvalue_5))
    (:NewEnumerator5
      (bind _returnvalue_6 (Game|SpawnActorfromClass "/Game/Blueprints/Player/BP_PerformerBase.BP_PerformerBase_C" Loc "Undefined" (Pawn|GetController) _playernumber 0))
      (Pawn|Possess (Game|GetPlayerController _playernumber) _returnvalue_6))
    (:NewEnumerator6
      (bind _returnvalue_7 (Game|SpawnActorfromClass "/Game/Blueprints/Player/BP_PerformerBase.BP_PerformerBase_C" Loc "Undefined" (Pawn|GetController) _playernumber 0))
      (Pawn|Possess (Game|GetPlayerController _playernumber) _returnvalue_7))))