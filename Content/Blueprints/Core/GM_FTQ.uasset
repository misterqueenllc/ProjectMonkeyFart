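; GM_FTQ appears to be a game mode for local multiplayer fights with a shared camera, but its BeginPlay and Tick are empty.
; Disconnected legacy graphs create one to four players, point two controllers at BP_FightCamera, and center it between two performers with distance-based boom length.
; The GetAllPlayers function, uncalled here, assigns the first CH_PerformerBase found to both Player1 and Player2.
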(event EventBeginPlay)

(event EventTick
  (params (DeltaSeconds :type Float%20%28single-precision%29)))

(fn ConstructionScript)

(fn GetAllPlayers
  (bind _outactors (Actor|GetAllActorsOfClass "/Game/Blueprints/Player/CH_PerformerBase.CH_PerformerBase_C"))
  (Variables|Default|SetPlayer1 (Utilities|Array|Get(acopy) _outactors))
  (Variables|Default|SetPlayer2 (Utilities|Array|Get(acopy) _outactors)))