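; Game mode for a performer fighting match with Stock or Time rules and a sudden death event setting every performer to 300 percent.
; BeginPlay creates offline local players from GameInstance character picks, copying stock count and minutes.
; GameEnd nudges time dilation toward slow motion, then copies match stats to the GameInstance.
; Tick is empty: countdown, end-condition and all-loaded checks are disconnected, as are VictoryScreen travel calls.
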(event Custom|GameEnd
  (bind _instance (Variables|Default|GetInstance))
  ;[1 0.5 0 1 30] End Game
  (Variables|/Game/Blueprints/Core/GI_PerformanceInstance.GI_PerformanceInstance_C|SetEndGame (Variables|Default|GetInstance) true)
  (Utilities|FlowControl|Delay 0.01)
  (Utilities|Time|SetGlobalTimeDilation (Math|Interpolation|FInterpTo (Class|GameplayStatics|GetGlobalTimeDilation) 0.1 (Variables|Default|GetDelta) 1.0))
  (Utilities|FlowControl|Delay 2.0)
  (Variables|/Game/Blueprints/Core/GI_PerformanceInstance.GI_PerformanceInstance_C|SetElims _instance (Variables|Stats|GetElims))
  (Variables|/Game/Blueprints/Core/GI_PerformanceInstance.GI_PerformanceInstance_C|SetFalls _instance (Variables|Stats|GetFalls))
  (Variables|/Game/Blueprints/Core/GI_PerformanceInstance.GI_PerformanceInstance_C|SetDmgDone _instance (Variables|Stats|GetDamageDone))
  (Variables|/Game/Blueprints/Core/GI_PerformanceInstance.GI_PerformanceInstance_C|SetDmgTaken _instance (Variables|Stats|GetDamageTaken))
  (if (Variables|/Game/Blueprints/Core/GI_PerformanceInstance.GI_PerformanceInstance_C|GetOnline _instance)
    (Development|PrintString "EndGame")))

(event Custom|CreatePlayers
  ;[1 1 0 1 30] CreatePlayers
  (Actor|GetAllActorsOfClass "/Game/Blueprints/LevelObjects/BP_Spawn.BP_Spawn_C")
  (bind _asgi_performance_instance (Utilities|Casting|CastToGI_PerformanceInstance (Game|GetGameInstance)))
  (bind _output_get (Variables|Default|SetInstance _asgi_performance_instance))
  (Variables|Stats|SetNoOfPlayers (Variables|/Game/Blueprints/Core/GI_PerformanceInstance.GI_PerformanceInstance_C|GetNumberofPlayers _output_get))
  (if (not (Variables|/Game/Blueprints/Core/GI_PerformanceInstance.GI_PerformanceInstance_C|GetOnline _output_get))
    (for (_array_element _array_index) (Variables|/Game/Blueprints/Core/GI_PerformanceInstance.GI_PerformanceInstance_C|GetPlayerCharacters _output_get)
      (if (Utilities|Enum|NotEqual(Enum) _array_element "NewEnumerator0")
        (Class|GameplayStatics|CreatePlayer _array_index)
        (Development|PrintString (Utilities|String|Append (Utilities|String|ToString(Integer) _array_index) "Player Created") true true "(R=0.104136,G=0.030858,B=1.000000,A=1.000000)" 2e+01)
        (Game|Feedback|PlayDynamicForceFeedback (Game|GetPlayerController _array_index) 4.0 0.3 true true true true)
        (Utilities|Array|SetArrayElem (Variables|Stats|GetStocks) _array_index (Variables|/Game/Blueprints/Core/GI_PerformanceInstance.GI_PerformanceInstance_C|GetStockCount (Variables|Default|GetInstance)))
        (Development|PrintString (Utilities|String|Append (Utilities|String|ToString(Integer) _array_index) " Stocks Created") true true "(R=1.000000,G=0.511704,B=0.043877,A=1.000000)" 2e+01)
        (Variables|Time|SetMin (Variables|/Game/Blueprints/Core/GI_PerformanceInstance.GI_PerformanceInstance_C|GetMin (Variables|Default|GetInstance)))))))

(event Custom|SetStocks
  ;[1 1 0 1 30] Set Player Stocks
  (if (Utilities|Enum|Equal(Enum) (Variables|Default|GetMode) "NewEnumerator0")
    (for _index (range 0 (Variables|Stats|GetNoOfPlayers))
      (Utilities|Array|SetArrayElem (Variables|Stats|GetStocks) _index (Variables|/Game/Blueprints/Core/GI_PerformanceInstance.GI_PerformanceInstance_C|GetStockCount (Variables|Default|GetInstance)) true))))

(event Custom|SuddenDeath
  ;[1 1 1 1 30] suddenDeath
  (Utilities|FlowControl|DoOnce false
    (:Completed
      (bind _outactors (Actor|GetAllActorsOfClass "/Game/Blueprints/Player/BP_PerformerBase.BP_PerformerBase_C"))
      (for _array_element _outactors
        (Variables|/Game/Blueprints/Player/Components/BPC_BP_CharacterStats.BPC_BP_CharacterStats_C|SetPercent (Variables|/Game/Blueprints/Player/BP_PerformerBase.BP_PerformerBase_C|GetCharacterStats _array_element) 300)))))

(event Custom|OnlineLoaded
  ;[1 1 0 1 30] All Online Players Have Loaded
  (Utilities|FlowControl|Delay 0.01)
  (bind _asgi_performance_instance (Utilities|Casting|CastToGI_PerformanceInstance (Game|GetGameInstance)))
  (for _index (range 0 (Variables|/Game/Blueprints/Core/GI_PerformanceInstance.GI_PerformanceInstance_C|GetNumberofPlayers _asgi_performance_instance))
    (Utilities|Array|SetArrayElem (Variables|Default|GetPlayerLoaded) _index false true)))

(event Custom|MatchStats
  ;[1 1 0 1 30] MatchStats
  (Variables|Stats|SetPlayersAlive (Variables|Stats|GetNoOfPlayers)))

(event EventTick
  (params (DeltaSeconds :type Float%20%28single-precision%29))
  ;[1 1 0 1 30] Tick
)

(event EventBeginPlay
  ;[1 1 0 1 30] BeginPlay
  (CallFunction|CreatePlayers)
  (CallFunction|OnlineLoaded)
  (CallFunction|MatchStats)
  (if (Utilities|Enum|Equal(Enum) (Variables|Default|GetMode) "NewEnumerator1")
    (Variables|Default|SetTimer true)
    (else
      (Variables|Default|SetTimer false))))

(fn ConstructionScript)

(fn FuncEndGameCondition
  (switch Utilities|FlowControl|Switch|SwitchonE_GameSubType (Variables|Default|GetMode)
    (:NewEnumerator0
      ;[1 1 1] StockMode
      (if (== (Variables|Stats|GetPlayersAlive) 1)
        (CallFunction|GameEnd)))
    (:NewEnumerator1
      ;[1 1 1] TimeMode
      (if (< (Variables|Time|GetMin) 0)
        (Variables|Default|SetTimer false)
        (CallFunction|GameEnd)))))

(fn FuncTimer
  (if (Variables|Default|GetTimer)
    (Utilities|FlowControl|Sequence
      (:then_0
        (bind _output_get (Variables|Time|SetSeconds (- (Variables|Time|GetSeconds) (Variables|Default|GetDelta))))
        (if (> (Math|Float|Round _output_get) 9)
          (Variables|Default|SetTimerText (Utilities|String|Append (Utilities|String|Append (Utilities|String|ToString(Integer) (Variables|Time|GetMin)) ":") (Utilities|String|ToString(Integer) (Math|Float|Round _output_get))))
          (else
            (Variables|Default|SetTimerText (Utilities|String|Append (Utilities|String|Append (Utilities|String|Append (Utilities|String|ToString(Integer) (Variables|Time|GetMin)) ":") "0") (Utilities|String|ToString(Integer) (Math|Float|Round _output_get)))))))
      (:then_1
        (if (<= (Variables|Time|GetSeconds) 0.0)
          (Variables|Time|SetSeconds 6e+01)
          (Math|Integer|DecrementInt (Variables|Time|GetMin)))))))