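; Menu game mode that handles per-player navigation for the main, character select and map select screens, then loads the chosen level.
; It reads GameType and the current menu from GI_PerformanceInstance on BeginPlay.
; Direction events switch on that menu, stepping MenuNumber or per-player row and column arrays through helper functions, with click sounds.
; Selecting locks a player's character cursor; GameStart opens Moodz, even for Random, and MenuStart is an empty switch.
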(event Custom|SelectSound
  ;[1 1 0 1 30] Play Sounds
  (Audio|PlaySound2D 0 1.0 1.0 0.0 0 0))

(event Custom|GameStart
  ;[1 1 0 1 30] Load Map
  (Variables|Default|SetStart true)
  (switch Utilities|FlowControl|Switch|SwitchonE_Maps (Variables|Default|GetMap)
    (:NewEnumerator0
      (Game|OpenLevel(byName) "Moodz" :!label _label))
    (:NewEnumerator1
      (switch int (Math|Random|RandomInteger 2)
        (:0
          (goto _label))
        (:1
          (Game|OpenLevel(byName) "Moodz"))
        (:2
          (Game|OpenLevel(byName) "Moodz"))))))

(event Custom|RightEvent
  (params (PlayerNo :type Integer))
  ;[1 1 0 1 30] Right Direction
  (switch Utilities|FlowControl|Switch|SwitchonE_Menus (Variables|Default|GetMenus)
    (:NewEnumerator1
      (if (not (Utilities|Array|Get(acopy) (Variables|Player|GetPlayerSelected) PlayerNo))
        (Utilities|AddtoArray (Variables|Default|GetColumns) PlayerNo :!label _label)
        (CallFunction|MenuClickSound)))
    (:NewEnumerator2
      (goto _label))))

(event Custom|UpEvent
  (params (PlayerNo :type Integer))
  ;[1 1 0 1 30] Press Up
  (switch Utilities|FlowControl|Switch|SwitchonE_Menus (Variables|Default|GetMenus)
    (:NewEnumerator0
      (Variables|Default|SetMenuNumber (- (Variables|Default|GetMenuNumber) 1))
      (CallFunction|MenuClickSound))
    (:NewEnumerator1
      (if (not (Utilities|Array|Get(acopy) (Variables|Player|GetPlayerSelected) PlayerNo))
        (Utilities|SubtractfromArray (Variables|Default|GetRows) PlayerNo :!label _label)
        (CallFunction|MenuClickSound)))
    (:NewEnumerator2
      (goto _label))))

(event Custom|DownEvent
  (params (PlayerNo :type Integer))
  ;[1 1 0 1 30] Press Down
  (switch Utilities|FlowControl|Switch|SwitchonE_Menus (Variables|Default|GetMenus)
    (:NewEnumerator0
      (Variables|Default|SetMenuNumber (+ (Variables|Default|GetMenuNumber) 1))
      (CallFunction|MenuClickSound))
    (:NewEnumerator1
      (if (not (Utilities|Array|Get(acopy) (Variables|Player|GetPlayerSelected) PlayerNo))
        (Utilities|SubtractfromArray (Variables|Default|GetRows) PlayerNo :!label _label)
        (CallFunction|MenuClickSound)))
    (:NewEnumerator2
      (goto _label))))

(event Custom|MenuStart
  ;[1 1 0 1 30] Start Action
  (switch Utilities|FlowControl|Switch|SwitchonE_Menus (Variables|Default|GetMenus)))

(event Custom|LeftEvent
  (params (PlayerNo :type Integer))
  ;[1 1 0 1 30] Left Direction
  (switch Utilities|FlowControl|Switch|SwitchonE_Menus (Variables|Default|GetMenus)
    (:NewEnumerator1
      (if (not (Utilities|Array|Get(acopy) (Variables|Player|GetPlayerSelected) PlayerNo))
        (Utilities|SubtractfromArray (Variables|Default|GetColumns) PlayerNo :!label _label)
        (CallFunction|MenuClickSound)))
    (:NewEnumerator2
      (goto _label))))

(event Custom|MenuClickSound
  ;[1 1 0 1 30] Play Sounds
  (Audio|PlaySound2D 0 1.0 1.0 0.0 0 0))

(event Custom|MenuAction
  (params (Player :type Integer))
  (bind _playerselected (Variables|Player|GetPlayerSelected))
  ;[1 1 0 1 30] Select Action
  (switch Utilities|FlowControl|Switch|SwitchonE_Menus (Variables|Default|GetMenus)
    (:NewEnumerator1
      (if (not (Utilities|Array|Get(acopy) _playerselected Player))
        (Utilities|Array|SetArrayElem _playerselected Player false)))))

(event EventBeginPlay
  ;[1 1 0 1 30] BeginPlay
  (bind _asgi_performance_instance (Utilities|Casting|CastToGI_PerformanceInstance (Game|GetGameInstance)))
  (bind _output_get (Variables|Default|SetGameInstance _asgi_performance_instance))
  (Variables|Default|SetGameType (Variables|/Game/Blueprints/Core/GI_PerformanceInstance.GI_PerformanceInstance_C|GetGameType _output_get))
  (Variables|Default|SetMenus (Variables|/Game/Blueprints/Core/GI_PerformanceInstance.GI_PerformanceInstance_C|GetMenus _output_get)))

(fn ConstructionScript)