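; Game state for a multiplayer match that tracks player deaths and ends the game in Stock or Time mode.
; Tick checks for one survivor or an expired countdown, which also builds timer text and scores players as eliminations minus falls.
; Game end records the winner from the alive array, then sets an end flag and lowers global time dilation through server and online-client events.
; The victory-screen level change and score-based ranking are unconnected.
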(event Custom|GameEnd
  ;[1 0.8394 0.1886 1 30] End Game
  (Utilities|FlowControl|DoOnce false
    (:Completed
      (CallFunction|FSetWinner)
      (CallFunction|EndGameServer)
      (if (Variables|/Game/Blueprints/Core/GI_PerformanceInstance.GI_PerformanceInstance_C|GetOnline (Variables|Default|GetInstance))
        (CallFunction|EndGameClients)))))

(event Custom|EndGameServer
  ;[1 0.8394 0.1886 1 30] End Game
  (Variables|/Game/Blueprints/Core/GI_PerformanceInstance.GI_PerformanceInstance_C|SetEndGame (Variables|Default|GetInstance) true)
  (Utilities|FlowControl|Delay 0.01)
  (Utilities|Time|SetGlobalTimeDilation (Math|Interpolation|FInterpTo (Class|GameplayStatics|GetGlobalTimeDilation) 0.1 (Variables|Default|GetDelta) 1.0))
  (Utilities|FlowControl|Delay 2.0)
  (if (Variables|/Game/Blueprints/Core/GI_PerformanceInstance.GI_PerformanceInstance_C|GetOnline (Variables|Default|GetInstance))
    (Development|PrintString "Victory")
    (else
      (Development|PrintString "Victory"))))

(event Custom|OnlineLoaded
  ;[1 0.581 0.966 1 30] All Online Players Have Loaded
  (Utilities|FlowControl|Delay 0.01)
  (for _index (range 0 (Variables|/Game/Blueprints/Core/GI_PerformanceInstance.GI_PerformanceInstance_C|GetNumberofPlayers (Variables|Default|GetInstance)))
    (Utilities|Array|SetArrayElem (Variables|Default|GetPlayerLoaded) _index false true)))

(event Custom|PlayerDeath
  (params (PlayerNo :type Integer))
  (CallFunction|FPlayerDeath PlayerNo))

(event Custom|EndGameClients
  ;[1 0.8394 0.1886 1 30] End Game
  (Variables|/Game/Blueprints/Core/GI_PerformanceInstance.GI_PerformanceInstance_C|SetEndGame (Variables|Default|GetInstance) true)
  (Utilities|FlowControl|Delay 0.01)
  (Utilities|Time|SetGlobalTimeDilation (Math|Interpolation|FInterpTo (Class|GameplayStatics|GetGlobalTimeDilation) 0.1 (Variables|Default|GetDelta) 1.0)))

(event EventBeginPlay
  ;[0.5535 1 0.2465 1 30] BeginPlay
  (bind _asgi_performance_instance (Utilities|Casting|CastToGI_PerformanceInstance (Game|GetGameInstance)))
  (Variables|Default|SetInstance _asgi_performance_instance)
  (bind _asgm_performance_mode (Utilities|Casting|CastToGM_PerformanceMode (Game|GetGameMode)))
  (Variables|Default|SetGameMode _asgm_performance_mode)
  (CallFunction|OnlineLoaded)
  (if (Utilities|Enum|Equal(Enum) (Variables|Default|GetMode) "NewEnumerator1")
    (Variables|Default|SetTimer true)
    (else
      (Variables|Default|SetTimer false))))

(event EventTick
  (params (DeltaSeconds :type Float%20%28single-precision%29))
  ;[1 1 1 1 30] Tick
  (Variables|Default|SetDelta DeltaSeconds)
  (Utilities|FlowControl|Sequence
    (:then_0
      (CallFunction|FEndGame)
      (CallFunction|FTimer))
    (:then_1
      (if (not (Utilities|Array|ContainsItem (Variables|Default|GetPlayerLoaded) false))
        (Variables|Default|SetAllLoaded true)))))

(fn ConstructionScript)

(fn FPlayerDeath
  (params (PlayerNo :type Integer))
  (bind _instance (Variables|Default|GetInstance))
  (Utilities|Array|SetArrayElem (Variables|/Game/Blueprints/Core/GI_PerformanceInstance.GI_PerformanceInstance_C|GetAliveArray _instance) PlayerNo false)
  (Utilities|Array|Insert (Variables|/Game/Blueprints/Core/GI_PerformanceInstance.GI_PerformanceInstance_C|GetPlayerPositions _instance) PlayerNo)
  (Variables|/Game/Blueprints/Core/GI_PerformanceInstance.GI_PerformanceInstance_C|SetPlayersAlive _instance (- (Variables|/Game/Blueprints/Core/GI_PerformanceInstance.GI_PerformanceInstance_C|GetPlayersAlive _instance) 1)))

(fn FEndGame
  (switch Utilities|FlowControl|Switch|SwitchonE_GameSubType (Variables|Default|GetMode)
    (:NewEnumerator0
      ;[1 1 1] StockMode
      (if (== (Variables|/Game/Blueprints/Core/GI_PerformanceInstance.GI_PerformanceInstance_C|GetPlayersAlive (Variables|Default|GetInstance)) 1)
        (CallFunction|GameEnd)))
    (:NewEnumerator1
      ;[1 1 1] TimeMode
      (if (< (Variables|Default|GetMin) 0)
        (Variables|Default|SetTimer false)
        (CallFunction|GameEnd)))))

(fn FSetWinner
  (bind _instance (Variables|Default|GetInstance))
  (bind _playerpositions (Variables|/Game/Blueprints/Core/GI_PerformanceInstance.GI_PerformanceInstance_C|GetPlayerPositions _instance))
  (for (_array_element _array_index) (Variables|/Game/Blueprints/Core/GI_PerformanceInstance.GI_PerformanceInstance_C|GetAliveArray (Variables|Default|GetInstance))
    (if (Math|Boolean|Equal(Boolean) _array_element true)
      (bind _output_get (Variables|/Game/Blueprints/Core/GI_PerformanceInstance.GI_PerformanceInstance_C|SetWinner _instance _array_index))
      (Utilities|Array|Insert _playerpositions 0 _output_get)
      (Utilities|Array|SetArrayElem _playerpositions 0 _output_get true))))

(fn FTimer
  (if (Variables|Default|GetTimer)
    (CallFunction|FTimerPositions)
    (Utilities|FlowControl|Sequence
      (:then_0
        (bind _output_get (Variables|Default|SetSeconds (- (Variables|Default|GetSeconds) (Variables|Default|GetDelta))))
        (if (> (Math|Float|Round _output_get) 9)
          (Variables|Default|SetTimerText (Utilities|String|Append (Utilities|String|Append (Utilities|String|ToString(Integer) (Variables|Default|GetMin)) ":") (Utilities|String|ToString(Integer) (Math|Float|Round _output_get))))
          (else
            (Variables|Default|SetTimerText (Utilities|String|Append (Utilities|String|Append (Utilities|String|Append (Utilities|String|ToString(Integer) (Variables|Default|GetMin)) ":") "0") (Utilities|String|ToString(Integer) (Math|Float|Round _output_get)))))))
      (:then_1
        (if (<= (Variables|Default|GetSeconds) 0.0)
          (Variables|Default|SetSeconds 6e+01)
          (Math|Integer|DecrementInt (Variables|Default|GetMin)))))))

(fn FTimerPositions
  (for _index (range 0 (Variables|Default|GetPlayersAlive))
    (Utilities|Array|SetArrayElem (Variables|/Game/Blueprints/Core/GI_PerformanceInstance.GI_PerformanceInstance_C|GetScore (Variables|Default|GetInstance)) _index (- (Utilities|Array|Get(acopy) (Variables|Default|GetElims) _index) (Utilities|Array|Get(acopy) (Variables|Default|GetFalls) _index)) true)))